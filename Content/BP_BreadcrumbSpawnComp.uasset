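; An actor component that drops a trail of BP_Breadcrumb actors behind its owner.
; A looping timer started on BeginPlay spawns each breadcrumb slightly behind the owner along its forward vector, matching its rotation and scale, then sets the breadcrumb's lifetime.
; StopSpawning is checked after each spawn and clears the timer, so one last breadcrumb appears after it is set.
; A BeginLife call on the breadcrumb is left unconnected.
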(event EventBeginPlay
  (bind _returnvalue (Utilities|Time|SetTimerbyFunctionName 0 "TimerComplete" (Variables|Default|GetTimeTilSpawn) true))
  (Variables|Default|SetTimerHandle _returnvalue))

(event EventTick
  (params (DeltaSeconds :type Float%20%28single-precision%29)))

(fn TimerComplete
  (bind _returnvalue (Components|GetOwner))
  (bind _returnvalue_2 (Transformation|GetActorTransform _returnvalue))
  (bind _returnvalue_3 (Game|SpawnActorfromClass "/Game/Ch_4/Actors/Player/BP_Breadcrumb.BP_Breadcrumb_C" (Math|Transform|MakeTransform (+ (* (Transformation|GetActorForwardVector _returnvalue) -5e+01) (.location _returnvalue_2)) (.rotation _returnvalue_2) (.scale _returnvalue_2)) "Undefined" 0 0))
  (Default|SetLifetime _returnvalue_3 (Variables|Default|GetBreadcrumbLifetime))
  (if (Variables|Default|GetbStopSpawning)
    (Utilities|Time|ClearandInvalidateTimerbyHandle (Variables|Default|GetTimerHandle))))